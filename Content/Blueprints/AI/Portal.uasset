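; Enemy spawn portal that reveals its Niagara effect once the game mode's Seconds passes 75600 (21:00, if counted from midnight).
; Spawn loops over Wave entries, creating the requested number of Golems or Champipis at the portal, passing the core position only to Golems.
; Each spawn increments the game mode's NbGolemsLeft, whatever the enemy type.
; The between-wave delay is disconnected, so all waves spawn at once.
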(event `self.ReceiveTick`
  (params (DeltaSeconds :type "Float (single-precision)"))
  (bind _asdemain_game_mode (cast `/Game/Blueprints/Game/DemainGameMode` (`GameplayStatics.GetGameMode`)))
  (if (> (`/Game/Blueprints/Game/DemainGameMode.seconds` _asdemain_game_mode) 75600.0)
    (`SceneComponent.SetVisibility` (`self.Niagara`) true false)))

(event `Spawn`
  (params (CorePos :type "Transform Structure"))
  (bind _returnvalue (`self.GetTransform`))
  (for _array_element (`self.Wave`)
    (bind (_enemytospawn _numbertospawn _delaybeforenextwave) (break `/Game/Blueprints/AI/S_Wave` _array_element))
    (for _ (range _numbertospawn)
      (bind _asdemain_game_mode (cast `/Game/Blueprints/Game/DemainGameMode` (`GameplayStatics.GetGameMode`)))
      (`/Engine/EditorBlueprintResources/StandardMacros.IncrementInt` (`/Game/Blueprints/Game/DemainGameMode.NbGolemsLeft` _asdemain_game_mode)
        (:`  `
          (`KismetSystemLibrary.PrintString` "SPAAAWWWNNN")
          (switch `/Game/Blueprints/AI/EnemyList` _enemytospawn
            (:`NewEnumerator0`
              (`|SpawnActorFromClass` "/Game/Blueprints/AI/Golem/BP_Golem.BP_Golem_C" _returnvalue "Undefined" "OverrideRootScale" null CorePos null))
            (:`NewEnumerator1`
              (`|SpawnActorFromClass` "/Game/Blueprints/AI/Champis/BP_BaseChampi.BP_BaseChampi_C" _returnvalue "Undefined" "OverrideRootScale" null null))))))))

(fn `UserConstructionScript`)