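; Health component that tracks its owner's health, starting at MaxHealth, with damage, healing capped at max, and death.
; GetsHurt subtracts damage, plays a sound and casts the owner to Golem, Echo or Champi for damage reactions, through sequence branches that can repeat the Echo and death checks.
; At zero health, a Core corrupts instead of dying; others receive BPI_DeathEvent's DeathMessage if implemented, otherwise DemainGameMode's GameOver is called.
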(event `self.ReceiveBeginPlay`
  (set `self.Health` (`self.MaxHealth`)))

(fn `Death:x`
  (bind _returnvalue (`self.GetOwner`))
  (bind _asdemain_game_mode (cast `/Game/Blueprints/Game/DemainGameMode` (`GameplayStatics.GetGameMode`)))
  (if (`KismetSystemLibrary.DoesImplementInterface` _returnvalue "/Game/Blueprints/AI/BPI_DeathEvent.BPI_DeathEvent_C")
    (message `/Game/Blueprints/AI/BPI_DeathEvent.Death` _returnvalue)
    (else
      (`/Game/Blueprints/Game/DemainGameMode.GameOver` _asdemain_game_mode _returnvalue))))

(fn `GetsHealed`
  (params (HealthBack :type "Float (double-precision)"))
  (bind _returnvalue (+ (`self.Health`) HealthBack))
  (if (>= _returnvalue (`self.MaxHealth`))
    (set `self.Health` (`self.MaxHealth`))
    (else
      (set `self.Health` _returnvalue))))

(fn `GetsHurt`
  (params (Damage :type "Float (double-precision)"))
  (bind _returnvalue (`self.GetOwner`))
  (`GameplayStatics.PlaySoundAtLocation` "/Game/Tech/Sons/Sound_design/Coup_d_pelle.Coup_d_pelle" (0.0 0.0 0.0) (struct) 1.0 1.0 0.0 null null null)
  (bind _output_get (set `self.Health` (- (`self.Health`) Damage)))
  (`|ExecutionSequence`
    (:`then_0`
      (`KismetSystemLibrary.PrintString` (`KismetStringLibrary.Concat_StrStr` (`KismetSystemLibrary.GetDisplayName` (`self.GetOwner`)) "' health: " (`KismetStringLibrary.Conv_DoubleToString` 0.0)))
      (bind _asbp_golem (cast `/Game/Blueprints/AI/Golem/BP_Golem` _returnvalue)
        (:`then`
          (`/Game/Blueprints/AI/Golem/BP_Golem.GolemDamage` _asbp_golem))
        (:`CastFailed`
          (bind _asbp_echo (cast `/Game/Blueprints/Player/BP_Echo` _returnvalue :!label _label)
            (:`then`
              (`/Game/Blueprints/Player/BP_Echo.EchoDamage` _asbp_echo)
              (`/Game/Blueprints/Player/BP_Echo.GetHurt` _asbp_echo))
            (:`CastFailed`
              _))
          (if (<= (`self.Health`) 0.0)
            (set `self.Health` 0.0)
            ;[0.3465 1 0.01291] CoreDontDie
            (bind _asbp_core (cast `/Game/Blueprints/Core/BP_Core` (`self.GetOwner`))
              (:`then`
                (`/Game/Blueprints/Core/BP_Core.Corrupting` _asbp_core))
              (:`CastFailed`
                (`self.Death:x`)))))))
    (:`then_1`
      (`KismetSystemLibrary.PrintString` (`KismetStringLibrary.Concat_StrStr` (`KismetSystemLibrary.GetDisplayName` (`self.GetOwner`)) "' health: " (`KismetStringLibrary.Conv_DoubleToString` _output_get)))
      (bind _asbp_base_champi (cast `/Game/Blueprints/AI/Champis/BP_BaseChampi` _returnvalue)
        (:`then`
          (`/Game/Blueprints/AI/Champis/BP_BaseChampi.ChampiDamage` _asbp_base_champi))
        (:`CastFailed`
          (goto _label))))
    (:`then_2`
      (goto _label))))